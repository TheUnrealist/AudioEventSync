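; Balloon spawner actor for the sound sync demo that spawns an ItemClass actor on each SpawnBalloon call, tinted with the given color.
; Spawn location and yaw come from a fixed-seed random stream, scattered within MaxSpawnRadius of the spawner and flattened vertically.
; ApplyVelocity then adds mass-independent linear and angular impulses to the static mesh using unseeded randomness, so only placement is repeatable.
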(fn ConstructionScript
  (Math|Random|SetRandomStreamSeed (Variables|Default|GetRandomLocationStream) 10))

(fn SpawnBalloon
  (params (Color :type Vector))
  (bind _returnvalue (Game|SpawnActorfromClass (Variables|Default|GetItemClass) (Math|Transform|MakeTransform (+ (Transformation|GetWorldLocation (Variables|Default|GetDefaultSceneRoot)) (* (* (Math|Random|RandomUnitVectorfromStream (Variables|Default|GetRandomLocationStream)) (Variables|Default|GetMaxSpawnRadius)) "1.000000,1.000000,0.500000")) (Math|Rotator|MakeRotator 0.0 0.0 (Math|Random|RandomFloatinRangefromStream 0.0 3.6e+02 (Variables|Default|GetRandomLocationStream)))) "Undefined" 0 0))
  (Utilities|FlowControl|Sequence
    (:then_0
      (CallFunction|ApplyVelocity _returnvalue))
    (:then_1
      (bind _asbp_balloon (Utilities|Casting|CastToBP_Balloon _returnvalue))
      (Default|SetColor _asbp_balloon Color))))

(fn ApplyVelocity
  (params (Actor :type Actor%20Object%20Reference))
  (bind _returnvalue (Actor|GetComponentbyClass Actor "/Script/Engine.StaticMeshComponent"))
  (Class|PrimitiveComponent|AddAngularImpulse _returnvalue (* (Math|Random|RandomUnitVector) (Math|Random|RandomFloatinRange 0.3 0.6)) "None" true)
  (Physics|AddImpulse _returnvalue (* (Math|Random|RandomUnitVector) (Math|Random|RandomFloatinRange 1e+01 2e+01)) "None" true))